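; ShotTrigger is a trigger actor that costs the player a life when a tagged basketball overlaps it.
; On overlap it strips the ball's tag, resets the GS_Basketball score multiplier, decrements Lives and updates the multiplier display.
; At zero lives it opens MainMenu; otherwise it refreshes LivesDisplay and calls the ball's EventScored.
; BeginPlay seeds LivesDisplay from the game state.
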(event `self.ReceiveBeginPlay`
  (bind _asgs_basketball (cast `/Game/Blueprints/GS_Basketball` (`GameplayStatics.GetGameState`)))
  (`/Game/Blueprints/LivesDisplay.ChangeLives` (`self.Lives_Display`) (`/Game/Blueprints/GS_Basketball.Lives` _asgs_basketball)))

(event `self.ReceiveActorBeginOverlap`
  (params (OtherActor :type "Actor Object Reference"))
  (if (`self.ActorHasTag` OtherActor "Basketball")
    (bind _asbasketball (cast `/Game/Blueprints/Basketball` OtherActor))
    (`/Game/Blueprints/Basketball.RemoveTag` _asbasketball)
    (bind _asgs_basketball (cast `/Game/Blueprints/GS_Basketball` (`GameplayStatics.GetGameState`)))
    (bind _output_get (set `/Game/Blueprints/GS_Basketball.ScoreMultiplier` 1 _asgs_basketball))
    (`/Game/Blueprints/MultiplierDisp.ChangeMulti` (`self.MultiDis`) _output_get)
    (bind _output_get_2 (set `/Game/Blueprints/GS_Basketball.Lives` (- (`/Game/Blueprints/GS_Basketball.Lives` _asgs_basketball) 1) _asgs_basketball))
    (if (< _output_get_2 1)
      (`GameplayStatics.OpenLevel` "MainMenu")
      (else
        (`/Game/Blueprints/LivesDisplay.ChangeLives` (`self.Lives_Display`) _output_get_2)
        (`/Game/Blueprints/Basketball.Event Scored` _asbasketball)))))

(fn `UserConstructionScript`)