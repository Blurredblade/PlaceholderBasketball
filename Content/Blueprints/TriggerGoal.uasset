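; TriggerGoal is a goal trigger that awards points when an actor tagged Basketball overlaps it.
; On overlap it casts to Basketball and calls RemoveTag on the ball, then passes a three-point award through AddScore.
; The result goes to ScoreDis.ChangeScore for display, and the ball is notified through EventScored.
; The construction script initializes Score to zero.
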(event `self.ReceiveActorBeginOverlap`
  (params (OtherActor :type "Actor Object Reference"))
  (if (`self.ActorHasTag` OtherActor "Basketball")
    (bind _asbasketball (cast `/Game/Blueprints/Basketball` OtherActor))
    (`/Game/Blueprints/Basketball.RemoveTag` _asbasketball)
    (bind _new_score (`self.AddScore` 3))
    (`/Game/Blueprints/ScoreDisplay.ChangeScore` (`self.ScoreDis`) _new_score)
    (`/Game/Blueprints/Basketball.Event Scored` _asbasketball)))

(fn `AddScore`
  (params (Score :type Integer))
  (returns (`New Score` :type Integer))
  (bind _output_get (set `self.Score` (+ (stale _output_get) Score)))
  (return _output_get))

(fn `UserConstructionScript`
  (set `self.Score` 0))