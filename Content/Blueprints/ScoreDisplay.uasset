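; ScoreDisplay is an actor Blueprint that shows a score as text padded with leading zeros.
; Its ChangeScore function converts the given score to a string and prepends zeros in a loop when it is shorter than MinDigits.
; The result is set on ScoreNum; the event graph and construction script are empty, so updates happen only when ChangeScore is called.
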(fn `ChangeScore`
  (params (Score :type Integer))
  (bind _min_digits (`self.Min Digits`))
  ;[1 1 1] Changes Score with Leading Zeros
  (bind _output_get (set `self.TempString` (`KismetStringLibrary.Conv_IntToString` Score)))
  (bind _returnvalue (`KismetStringLibrary.Len` _output_get))
  (if (< _returnvalue _min_digits)
    (for _ (range (+ (- _min_digits _returnvalue) 1))
      (bind _output_get_2 (set `self.TempString` (`KismetStringLibrary.Concat_StrStr` "0" (stale _output_get_2))))))
  (`TextRenderComponent.K2_SetText` (`self.ScoreNum`) (`KismetTextLibrary.Conv_StringToText` _output_get_2)))

(fn `UserConstructionScript`)